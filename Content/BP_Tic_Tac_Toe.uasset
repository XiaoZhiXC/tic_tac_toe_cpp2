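; Tic-tac-toe game controller that creates the menu widgets, applies windowed display settings and runs matches against a computer opponent.
; The board is an array of vectors; GetFVector2D picks the computer's cell, BoradChange writes it, and IsGameOver triggers the result message and sound.
; Player input leads to a delayed computer reply, while a KeSuLu mode repeatedly fires computer moves from Tick.
; PlayMenuVioce switches between menu music and cycling game tracks.
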(event Custom|Cus_ComPlayFirst
  (bind _returnvalue (Class|MyPawn|GetFVector2D (Variables|Default|GetBorad)))
  (Math|Integer|DecrementInt (Variables|Default|GetCurrentDepth)
    (:%20%20
      (CallFunction|BoradChange (.x _returnvalue) (.y _returnvalue) -1.0)
      (Audio|PlaySound2D "/Game/Sounds/sfx/sfx_ui_02.sfx_ui_02" 1.0 1.0 0.0 0 0)
      (Variables|Default|SetIsManPlay true)
      (bind _returnvalue_2 (Class|MyPawn|IsGameOver (Variables|Default|GetBorad)))
      (if (!= _returnvalue_2 0)
        (Variables|Default|SetKeSuLuStart false)
        (bind _returnvalue_3 (UserInterface|CreateWidget "/Game/WB_Message.WB_Message_C" 0 (select (== _returnvalue_2 2) "平局！" (select (== _returnvalue_2 1) "你赢了！！" "你输了。。")) false))
        (UserInterface|Viewport|AddtoViewport _returnvalue_3 0)
        (Audio|PlaySound2D (select (== _returnvalue_2 1) "/Game/Sounds/music/win_Cue.win_Cue" "/Game/Sounds/music/lose_Cue.lose_Cue") 1.0 1.0 0.0 0 0)))))

(event Custom|Cus_PlayInputed
  (if (> (Variables|Default|GetCurrentDepth) 1)
    (Math|Integer|DecrementInt (Variables|Default|GetCurrentDepth)
      (:%20%20
        (Utilities|FlowControl|Delay 0.3)
        (bind _returnvalue (Class|MyPawn|GetFVector2D (Variables|Default|GetBorad)))
        (Math|Integer|DecrementInt (Variables|Default|GetCurrentDepth)
          (:%20%20
            (CallFunction|BoradChange (.x _returnvalue) (.y _returnvalue) -1.0)
            (Audio|PlaySound2D "/Game/Sounds/sfx/sfx_ui_02.sfx_ui_02" 1.0 1.0 0.0 0 0))))))
  (Variables|Default|SetIsManPlay true)
  (bind _returnvalue_2 (Class|MyPawn|IsGameOver (Variables|Default|GetBorad)))
  (if (!= _returnvalue_2 0)
    (Variables|Default|SetKeSuLuStart false)
    (bind _returnvalue_3 (UserInterface|CreateWidget "/Game/WB_Message.WB_Message_C" 0 (select (== _returnvalue_2 2) "平局！" (select (== _returnvalue_2 1) "你赢了！！" "你输了。。")) false))
    (UserInterface|Viewport|AddtoViewport _returnvalue_3 0)
    (Audio|PlaySound2D (select (== _returnvalue_2 1) "/Game/Sounds/music/win_Cue.win_Cue" "/Game/Sounds/music/lose_Cue.lose_Cue") 1.0 1.0 0.0 0 0)))

(event EventBeginPlay
  (bind _returnvalue (Game|GetPlayerController 0))
  (bind _returnvalue_2 (UserInterface|CreateWidget "/Game/WB_BackImage.WB_BackImage_C" _returnvalue))
  (Variables|Default|SetBackImgae _returnvalue_2)
  (UserInterface|Viewport|AddtoViewport _returnvalue_2 0)
  (bind _returnvalue_3 (UserInterface|CreateWidget "/Game/WB_GameStartSet.WB_GameStartSet_C" _returnvalue "Need to specify text"))
  (UserInterface|Viewport|AddtoViewport _returnvalue_3 0)
  (Variables|Default|SetDifficultLevel 2)
  (CallFunction|PlayMenuVioce true)
  (bind _returnvalue_4 (Settings|GetGameUserSettings))
  (Utilities|FlowControl|Sequence
    (:then_0
      (Class|GameUserSettings|SetFrameRateLimit _returnvalue_4 6e+01)
      (Class|GameUserSettings|ApplyNonResolutionSettings _returnvalue_4))
    (:then_1
      (Class|GameUserSettings|SetScreenResolution _returnvalue_4 (Utilities|Struct|MakeIntPoint 1280 720))
      (Class|GameUserSettings|SetFullscreenMode _returnvalue_4 "Windowed")
      (Class|GameUserSettings|ApplyResolutionSettings _returnvalue_4 true))))

(event Collision|EventActorBeginOverlap
  (params (OtherActor :type Actor%20Object%20Reference)))

(event EventTick
  (params (DeltaSeconds :type Float%20%28single-precision%29))
  (if (and (Variables|Default|GetIsKeSuLu) (Variables|Default|GetKeSuLuStart))
    (Utilities|FlowControl|Delay 0.05)
    (CallFunction|CusComPlayFirst)))

(fn ConstructionScript)

(fn BoradChange
  (params (InputX :type Integer) (InputY :type Integer) (ChangeValue :type Float%20%28double-precision%29))
  (LocalVariables|Setcopy (Utilities|Array|Get(acopy) (Variables|Default|GetBorad) InputX))
  (if (== InputY 0)
    (Utilities|Array|SetArrayElem (Variables|Default|GetBorad) InputX (Math|Vector|MakeVector ChangeValue (.y (LocalVariables|Getcopy)) (.z (LocalVariables|Getcopy))))
    (elif (== InputY 1)
      (Utilities|Array|SetArrayElem (Variables|Default|GetBorad) InputX (Math|Vector|MakeVector (.x (LocalVariables|Getcopy)) ChangeValue (.z (LocalVariables|Getcopy))))
      (else
        (Utilities|Array|SetArrayElem (Variables|Default|GetBorad) InputX (Math|Vector|MakeVector (.x (LocalVariables|Getcopy)) (.y (LocalVariables|Getcopy)) ChangeValue))))))

(fn Inital
  (Variables|Default|SetBorad (Variables|Default|GetEmptyBorad))
  (Variables|Default|SetCurrentDepth 9)
  (Variables|Default|SetIsManPlay true))

(fn PlayMenuVioce
  (params (IsMenu :type Boolean))
  (bind _gamebgm (Variables|Default|GetGameBgm))
  (if IsMenu
    (bind _returnvalue (Audio|CreateSound2D "/Game/Sounds/music/menu3_Cue.menu3_Cue" 1.0 1.0 0.0 0))
    (bind _output_get (Variables|Default|SetMenuComp _returnvalue))
    (Audio|Components|Audio|Play _output_get 0.0)
    (Utilities|IsValid (Variables|Default|GetGameBGMComp)
      (:Is%20Valid
        (Audio|Components|Audio|Stop (Variables|Default|GetGameBGMComp))))
    (else
      (bind _returnvalue_2 (Audio|CreateSound2D (Utilities|Array|Get(acopy) _gamebgm (Variables|Default|GetGameBgmIndex)) 1.0 1.0 0.0 0))
      (if (== (Variables|Default|GetGameBgmIndex) (- (Utilities|Array|Length _gamebgm) 1))
        (Variables|Default|SetGameBgmIndex 0)
        (else
          (Math|Integer|IncrementInt (Variables|Default|GetGameBgmIndex)
            (:%20%20
              _))))
      (bind _output_get_2 (Variables|Default|SetGameBGMComp _returnvalue_2))
      (Audio|Components|Audio|Play _output_get_2 0.0)
      (Utilities|IsValid (Variables|Default|GetMenuComp)
        (:Is%20Valid
          (Audio|Components|Audio|Stop (Variables|Default|GetMenuComp)))))))